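; PlayerBaseBP is a base player Blueprint that gives the player an on-screen HP bar, a brief text popup and keyboard-driven health changes.
; BeginPlay casts the controller to NP4HeroController and creates the HP bar widget, passing it the actor and controller.
; Releasing T briefly shows a ShowText widget, gated by CanShowText against overlap.
; K heals up to HealthMax, while a second T-press binding subtracts health without clamping.
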(event EventActorBeginOverlap
  (params (OtherActor :type Actor%20Object%20Reference)))

(event EventTick
  (params (DeltaSeconds :type Float%20%28single-precision%29)))

(event EventBeginPlay
  ;[1 1 1] set : Player Actor & controller
  (Variables|Default|SetMyPlayerBP self)
  (Variables|Default|SetMyPlayerActor self)
  (bind _asnp4hero_controller (Utilities|Casting|CastToNP4HeroController (Game|GetPlayerController 0))
    (:then
      (Variables|Default|SetMyPlayerController _asnp4hero_controller)
      (bind _returnvalue (UserInterface|CreateWidget "/Game/UI/PlayerHPBar.PlayerHPBar_C"))
      (bind _output_get (Variables|Default|SetHPBarWidget _returnvalue))
      (Variables|/Game/UI/PlayerHPBar.PlayerHPBar_C|SetHPActor _output_get (Variables|Default|GetMyPlayerActor))
      (Variables|/Game/UI/PlayerHPBar.PlayerHPBar_C|SetHPcontroller (Variables|Default|GetHPBarWidget) (Variables|Default|GetMyPlayerController))
      (UserInterface|Viewport|AddtoViewport (Variables|Default|GetHPBarWidget) 1))
    (:CastFailed
      (Development|PrintString 0 "Failed : Cast Controller in playerbaseBP"))))

(event Input|KeyboardEvents|T
  (params (Key :type Key%20Structure :default "AnyKey"))
  (bind _myplayerbp (Variables|Default|GetMyPlayerBP))
  (:Pressed
    (Variables|/Script/NP4.NP4CharacterBase|SetHealth _myplayerbp (- (Variables|/Script/NP4.NP4CharacterBase|GetHealth _myplayerbp) 1e+01))))

(event Input|KeyboardEvents|T
  (params (Key :type Key%20Structure :default "AnyKey"))
  (:Pressed
    (if (Variables|Default|GetCanShowText)
      (Development|PrintString 0 "T pressed" true true "(R=0.000000,G=0.660000,B=1.000000,A=1.000000)" 1.0)))
  (:Released
    (if (Variables|Default|GetCanShowText)
      (Development|PrintText 0 "T Released" true true "(R=0.000000,G=0.660000,B=1.000000,A=1.000000)" 1.0)
      (Variables|Default|SetCanShowText false)
      (bind _returnvalue (UserInterface|CreateWidget "/Game/UI/ShowText.ShowText_C"))
      (bind _output_get (Variables|Default|SetPlayerUpTextWidget _returnvalue))
      (Variables|/Game/UI/ShowText.ShowText_C|SetMyActor _output_get (Variables|Default|GetMyPlayerActor))
      (Variables|/Game/UI/ShowText.ShowText_C|SetMyController (Variables|Default|GetPlayerUpTextWidget) (Variables|Default|GetMyPlayerController))
      (Variables|/Game/UI/ShowText.ShowText_C|SetMyText (Variables|Default|GetPlayerUpTextWidget) (Variables|Default|GetPlayerUpText))
      (UserInterface|Viewport|AddtoViewport (Variables|Default|GetPlayerUpTextWidget) 1)
      (Utilities|FlowControl|Delay 0)
      (Widget|RemovefromParent (Variables|Default|GetPlayerUpTextWidget))
      (Variables|Default|SetCanShowText true))))

(event Input|KeyboardEvents|K
  (params (Key :type Key%20Structure :default "AnyKey"))
  (bind _myplayerbp (Variables|Default|GetMyPlayerBP))
  (bind _healthmax (Variables|/Script/NP4.NP4CharacterBase|GetHealthMax _myplayerbp))
  (:Pressed
    (if (<= (+ (Variables|/Script/NP4.NP4CharacterBase|GetHealth _myplayerbp) 1e+01) _healthmax)
      (Variables|/Script/NP4.NP4CharacterBase|SetHealth (Variables|Default|GetMyPlayerBP) (+ (Variables|/Script/NP4.NP4CharacterBase|GetHealth _myplayerbp) 1e+01))
      (else
        (Variables|/Script/NP4.NP4CharacterBase|SetHealth (Variables|Default|GetMyPlayerBP) _healthmax)))))

(fn ConstructionScript)